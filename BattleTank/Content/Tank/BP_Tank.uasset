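; Player tank Blueprint that registers its turret and barrel and handles orbit camera input.
; On BeginPlay it passes the Barrel and Turret components to setter functions.
; The TurretRight axis yaws the Gimbal, while TurretUp pitches the SpringArm within a clamped range, keeping yaw and pitch on separate components.
; Despite their names, these axes rotate only the camera rig here.
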(event EventBeginPlay
  (Class|Tank|SetBarrelComponent (Variables|Default|GetBarrel))
  (Class|Tank|SetTurretComponent (Variables|Default|GetTurret)))

(event Collision|EventActorBeginOverlap
  (params (OtherActor :type Actor%20Object%20Reference)))

(event EventTick
  (params (DeltaSeconds :type Float%20%28single-precision%29)))

(event Input|AxisEvents|InputAxisTurretRight
  (params (AxisValue :type Float%20%28single-precision%29))
  ;[1 1 1] Camera Movement
  (Transformation|AddRelativeRotation (Variables|Default|GetGimbal) (Math|Rotator|MakeRotator 0.0 0.0 AxisValue) false false))

(event Input|AxisEvents|InputAxisTurretUp
  (params (AxisValue :type Float%20%28single-precision%29))
  (bind _springarm (Variables|Default|GetSpringArm))
  ;[1 1 1] Camera Movement
  (Transformation|AddRelativeRotation _springarm (Math|Rotator|MakeRotator 0.0 AxisValue 0.0) false false)
  (Transformation|SetRelativeRotation _springarm (Math|Rotator|MakeRotator 0.0 (Math|Float|Clamp(Float) (.pitch (Variables|/Script/Engine.SceneComponent|GetRelativeRotation _springarm)) -5e+01 1e+01) 0.0) false false))

(fn ConstructionScript)